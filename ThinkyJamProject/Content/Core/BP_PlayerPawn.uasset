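; Player pawn Blueprint that switches the player's view between predefined camera positions, moving to an initial one on BeginPlay.
; LerpToCameraPosition searches CameraPositions for the entry matching the requested position enum and stores it as CurrentCameraPos.
; It then has the TJ player controller blend its view target to that entry with a short ease-in-out transition, even if no match updated it.
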(event EventBeginPlay
  (CallFunction|LerptoCameraPosition "NewEnumerator0"))

(event Collision|EventActorBeginOverlap
  (params (OtherActor :type Actor%20Object%20Reference)))

(event EventTick
  (params (DeltaSeconds :type Float%20%28single-precision%29)))

(fn ConstructionScript)

(fn LerptoCameraPosition
  (params (CameraPosition :type E_CameraPosition%20Enum :default "NewEnumerator0"))
  (bind _array_element (Utilities|Array|ForEachLoopwithBreak (Variables|Default|GetCameraPositions) :!label _label)
    (:LoopBody
      (if (Utilities|Enum|Equal(Enum) CameraPosition (Variables|/Game/Core/BP_CameraPosition.BP_CameraPosition_C|GetCameraPos _array_element))
        (Variables|Default|SetCurrentCameraPos _array_element)
        (goto _label Break)))
    (:Completed
      (Game|Player|SetViewTargetwithBlend (CallFunction|GetTJPlayerController) (Variables|Default|GetCurrentCameraPos) 0.6 "VTBlend_EaseInOut" 2.0 false))))