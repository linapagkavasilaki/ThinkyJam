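; BP_Evidence is a piece of evidence that can be dragged across a board with the mouse.
; Click and release toggle its drag state and register or clear it as the dragged evidence on the TJ player controller.
; While dragged, each tick traces under the cursor on a separate channel and places it slightly off the hit surface along the normal.
; Hovering shows a move tooltip, and BeginPlay caches its owner as the board.
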(event EventBeginPlay
  (Variables|Default|SetBoard (Components|GetOwner)))

(event Collision|EventActorBeginOverlap
  (params (OtherActor :type Actor%20Object%20Reference)))

(event EventTick
  (params (DeltaSeconds :type Float%20%28single-precision%29))
  (bind _tj_player_controller (CallFunction|GetTJPlayerController))
  (bind _hitresult (Game|Player|GetHitResultUnderCursorbyChannel _tj_player_controller "TraceTypeQuery3" true))
  (bind (_bblockinghit _binitialoverlap _time _distance _location _impactpoint _normal) (Collision|BreakHitResult _hitresult))
  (if (Variables|Default|GetIsBeingDragged)
    (if _bblockinghit
      (Transformation|SetActorLocation (+ _location (* _normal 2.0)) false false)
      (else
        (Development|PrintString "No board found")))))

(event MouseInput|EventActorOnClicked
  (params (ButtonPressed :type Key%20Structure :default "None"))
  (bind _tj_player_controller (CallFunction|GetTJPlayerController))
  (Variables|/Game/Core/TJ_PlayerController.TJ_PlayerController_C|SetDraggedEvidence _tj_player_controller self)
  (Variables|/Game/Core/TJ_PlayerController.TJ_PlayerController_C|SetDraggingEvidence _tj_player_controller true)
  (Variables|Default|SetIsBeingDragged true))

(event EventActorOnReleased
  (params (ButtonReleased :type Key%20Structure :default "None"))
  (bind _tj_player_controller (CallFunction|GetTJPlayerController))
  (Variables|/Game/Core/TJ_PlayerController.TJ_PlayerController_C|SetDraggedEvidence _tj_player_controller 0)
  (Variables|/Game/Core/TJ_PlayerController.TJ_PlayerController_C|SetDraggingEvidence _tj_player_controller false)
  (Variables|Default|SetIsBeingDragged false))

(event MouseInput|EventActorBeginCursorOver
  (CallFunction|ShowTooltipOverActor self "Click to move"))

(fn ConstructionScript)